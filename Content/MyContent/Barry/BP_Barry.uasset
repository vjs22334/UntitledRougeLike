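; BP_Barry is a character Blueprint that plays melee combo montages on left mouse click.
; An Attack flag gates input, while AttackCount selects one of three root montages and increments as each starts.
; Completion resets only the count; interruption waits on a retriggerable delay, then clears both.
; Attack is cleared nowhere else in this graph, and the other events just call their parents.
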(event `self.ReceiveBeginPlay`
  (`parent.ReceiveBeginPlay`))

(event `self.ReceiveTick`
  (params (DeltaSeconds :type "Float (single-precision)"))
  (`parent.ReceiveTick` DeltaSeconds))

(event `Key|LeftMouseButton`
  (params (Key :type "Key Structure"))
  (:`Pressed`
    (if (not (`self.Attack`))
      (set `self.Attack` true)
      (`|PlayMontage` (`self.Mesh`) (select `int` (`self.Attack Count`) :`0` "/Game/MyContent/Barry/Animation/Combo1_Attack1_Root_Montage.Combo1_Attack1_Root_Montage" :`1` "/Game/MyContent/Barry/Animation/Combo1_Attack2_Root_Montage.Combo1_Attack2_Root_Montage" :`2` "/Game/MyContent/Barry/Animation/Combo1_Attack4_Root_Montage.Combo1_Attack4_Root_Montage" :!type "AnimMontage Object Reference") 1.3
        (:`then`
          (`/Engine/EditorBlueprintResources/StandardMacros.IncrementInt` (`self.Attack Count`)))
        (:`OnCompleted`
          (set `self.Attack Count` 0 :!label _label))
        (:`OnInterrupted`
          (`KismetSystemLibrary.RetriggerableDelay` 1.5)
          (set `self.Attack` false)
          (goto _label))))))

(fn `UserConstructionScript`
  (`parent.UserConstructionScript`))